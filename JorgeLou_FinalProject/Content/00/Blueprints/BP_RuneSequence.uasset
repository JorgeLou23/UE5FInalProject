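; Rune trigger actor that runs a linked cinematic sequence while the Serath player character stands in its Activate volume.
; Entering plays the sequence at double speed; leaving pauses briefly, then plays it backward.
; The OnOff timeline scales Niagara effects and decal glow, with platform audio paused outside the volume.
; A looping, randomly offset timeline moves the mesh and recreates the decal's dynamic material every update.
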(event `self.ReceiveBeginPlay`
  (`|ExecutionSequence`
    (:`then_0`
      (bind (_direction _position) (`Timeline|Timeline_0` :`NewTime` (`KismetMathLibrary.RandomFloatInRange` 0.0 10.0) :!via `SetNewTime` :!label _label)
        (:`Update`
          (`SceneComponent.K2_SetRelativeLocation` (`self.StaticMesh`) (* _position (10.0 0.0 20.0)) false false)
          ;[1 1 1] CreateDynamicDecalMaterial
          (bind _returnvalue (`KismetMaterialLibrary.CreateDynamicMaterialInstance` "/Game/Isometric_World/Sky_Temple/Materials/Decals/MI_Decal_Temple_Symbol_11.MI_Decal_Temple_Symbol_11"))
          (set `self.DM_Decal` _returnvalue))
        (:`Finished`
          (`|ExecutionSequence`
            (:`then_0`
              (goto _label :!via `PlayFromStart`))))))
    (:`then_1`
      (goto _label))
    (:`then_2`
      (`AudioComponent.SetPaused` (`self.AudioPlatforms`) true))))

(event `self.Activate.OnComponentBeginOverlap`
  (params (OverlappedComponent :type "PrimitiveComponent Object Reference") (OtherActor :type "Actor Object Reference") (OtherComp :type "PrimitiveComponent Object Reference") (OtherBodyIndex :type Integer) (bFromSweep :type Boolean) (SweepResult :type "HitResult Structure (by ref)"))
  (cast `/Game/00/Characters/Serath/SerathPlayerCharacter` OtherActor)
  ;[1 1 1] PlayCall
  (`self.Start`)
  (`AudioComponent.SetPaused` (`self.AudioPlatforms`) false)
  ;[1 1 1] Activate/deactivate rune visual effects
  (bind (_direction _niagaradecalsrate) (`Timeline|OnOff` :!label _label_2)
    (:`Update`
      (`SceneComponent.SetWorldScale3D` (`self.Niagara`) (* _niagaradecalsrate (0.6 0.6 0.6)))
      (`MaterialInstanceDynamic.SetScalarParameterValue` (`self.DM_Decal`) "Emissive_Power" (* _niagaradecalsrate 100.0))
      (`DecalComponent.SetDecalMaterial` (`self.Decal`) (`self.DM_Decal`))
      (`DecalComponent.SetDecalMaterial` (`self.Decal1`) (`self.DM_Decal`))
      (`AudioComponent.Play` (`self.AudioPlatforms`) 0.0))))

(event `self.Activate.OnComponentEndOverlap`
  (params (OverlappedComponent :type "PrimitiveComponent Object Reference") (OtherActor :type "Actor Object Reference") (OtherComp :type "PrimitiveComponent Object Reference") (OtherBodyIndex :type Integer))
  (cast `/Game/00/Characters/Serath/SerathPlayerCharacter` OtherActor)
  ;[1 1 1] PlayCall
  (`self.Reverse`)
  (`AudioComponent.SetPaused` (`self.AudioPlatforms`) true)
  (goto _label_2 :!via `Reverse`))

(event `Start`
  (bind _sequenceplayer (`LevelSequenceActor.SequencePlayer` (`self.Cinematic`)))
  ;[1 1 1] PlayEvents
  (`MovieSceneSequencePlayer.SetPlayRate` _sequenceplayer 2.0)
  (`MovieSceneSequencePlayer.Play` _sequenceplayer))

(event `Reverse`
  (bind _sequenceplayer (`LevelSequenceActor.SequencePlayer` (`self.Cinematic`)))
  ;[1 1 1] PlayEvents
  (`MovieSceneSequencePlayer.Pause` _sequenceplayer)
  (`KismetSystemLibrary.Delay` 0.5)
  (`MovieSceneSequencePlayer.SetPlayRate` _sequenceplayer -1.0)
  (`MovieSceneSequencePlayer.Play` _sequenceplayer))

(fn `OnRep_Cinematic`)

(fn `UserConstructionScript`)