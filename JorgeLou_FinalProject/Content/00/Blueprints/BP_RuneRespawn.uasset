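; BP_RuneRespawn is a rune actor whose decals glow up when activated and fade back when deactivated.
; BeginPlay gathers seven decal components and creates a dynamic material instance for each.
; Activate plays a Timeline that drives the scaled Emissive_Power parameter on every instance and reassigns it to its decal each update.
; Deactivate runs the same Timeline in reverse from the end.
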(event `self.ReceiveBeginPlay`
  (bind _arraydecals (`self.ArrayDecals`))
  (`|ExecutionSequence`
    (:`then_0`
      (`KismetArrayLibrary.Array_Add` _arraydecals (`self.Decal`))
      (`KismetArrayLibrary.Array_Add` _arraydecals (`self.Decal1`))
      (`KismetArrayLibrary.Array_Add` _arraydecals (`self.Decal2`))
      (`KismetArrayLibrary.Array_Add` _arraydecals (`self.Decal3`))
      (`KismetArrayLibrary.Array_Add` _arraydecals (`self.Decal5`))
      (`KismetArrayLibrary.Array_Add` _arraydecals (`self.Decal6`))
      (`KismetArrayLibrary.Array_Add` _arraydecals (`self.Decal7`)))
    (:`then_1`
      (for _array_element (`self.ArrayDecals`)
        (bind _returnvalue (`DecalComponent.CreateDynamicMaterialInstance` _array_element))
        (`KismetArrayLibrary.Array_Add` (`self.DM_DecalArray`) _returnvalue)))))

(event `Activate`
  (bind (_direction _emmisive) (`Timeline|Timeline` :!via `PlayFromStart` :!label _label)
    (:`Update`
      (for (_array_element _array_index) (`self.DM_DecalArray`)
        (`MaterialInstanceDynamic.SetScalarParameterValue` _array_element "Emissive_Power" (* _emmisive 10.0))
        (`DecalComponent.SetDecalMaterial` (`|GetArrayItem` (`self.ArrayDecals`) _array_index) _array_element)))))

(event `Deactivate`
  (goto _label :!via `ReverseFromEnd`))

(fn `UserConstructionScript`)