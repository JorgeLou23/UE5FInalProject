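; BP_RuneEndLevel is an end-of-level rune that opens the end menu level when SerathPlayerCharacter overlaps its Sphere.
; The overlap calls Activate, which spins five rings through separate self-restarting timelines that add local rotation each update.
; Another timeline scales the static mesh and Niagara effect.
; The level opens immediately after Activate, as the two-second Delay leading to it is never triggered.
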(event `self.ReceiveBeginPlay`)

(event `Activate`
  (`|ExecutionSequence`
    (:`then_0`
      (bind (_direction _rotation) (`Timeline|Rotation` :!label _label)
        (:`Update`
          (`SceneComponent.K2_AddLocalRotation` (`self.Ring_01`) (`KismetMathLibrary.MakeRotator` (.x _rotation) (.y _rotation) (.z _rotation)) false false))
        (:`Finished`
          (`|ExecutionSequence`
            (:`then_0`
              (goto _label :!via `PlayFromStart`))))))
    (:`then_1`
      (bind (_direction_2 _rotation_2) (`Timeline|Timeline_0` :!label _label_2)
        (:`Update`
          (`SceneComponent.K2_AddLocalRotation` (`self.Ring_02`) (`KismetMathLibrary.MakeRotator` (.x _rotation_2) (.y _rotation_2) (.z _rotation_2)) false false))
        (:`Finished`
          (`|ExecutionSequence`
            (:`then_0`
              (goto _label_2 :!via `PlayFromStart`))))))
    (:`then_2`
      (bind (_direction_3 _rotation_3) (`Timeline|Timeline_1` :!label _label_3)
        (:`Update`
          (`SceneComponent.K2_AddLocalRotation` (`self.Ring_03`) (`KismetMathLibrary.MakeRotator` (.x _rotation_3) (.y _rotation_3) (.z _rotation_3)) false false))
        (:`Finished`
          (`|ExecutionSequence`
            (:`then_0`
              (goto _label_3 :!via `PlayFromStart`))))))
    (:`then_3`
      (bind (_direction_4 _rotation_4) (`Timeline|Timeline_2` :!label _label_4)
        (:`Update`
          (`SceneComponent.K2_AddLocalRotation` (`self.Ring_04`) (`KismetMathLibrary.MakeRotator` (.x _rotation_4) (.y _rotation_4) (.z _rotation_4)) false false))
        (:`Finished`
          (`|ExecutionSequence`
            (:`then_0`
              (goto _label_4 :!via `PlayFromStart`))))))
    (:`then_4`
      (bind (_direction_5 _rotation_5) (`Timeline|Timeline_3` :!label _label_5)
        (:`Update`
          (`SceneComponent.K2_AddLocalRotation` (`self.Ring_05`) (`KismetMathLibrary.MakeRotator` (.x _rotation_5) (.y _rotation_5) (.z _rotation_5)) false false))
        (:`Finished`
          (`|ExecutionSequence`
            (:`then_0`
              (goto _label_5 :!via `PlayFromStart`))))))
    (:`then_5`
      (bind (_direction_6 _active) (`Timeline|SphereNiagara`)
        (:`Update`
          (`SceneComponent.SetRelativeScale3D` (`self.StaticMesh`) (+ (* _active (0.5 0.5 0.5)) (0.2 0.2 0.2)))
          (`SceneComponent.SetRelativeScale3D` (`self.Niagara`) (* _active (1.428571 1.428571 1.428571))))))))

(event `self.Sphere.OnComponentBeginOverlap`
  (params (OverlappedComponent :type "PrimitiveComponent Object Reference") (OtherActor :type "Actor Object Reference") (OtherComp :type "PrimitiveComponent Object Reference") (OtherBodyIndex :type Integer) (bFromSweep :type Boolean) (SweepResult :type "HitResult Structure (by ref)"))
  (cast `/Game/00/Characters/Serath/SerathPlayerCharacter` OtherActor)
  (`self.Activate`)
  (`GameplayStatics.OpenLevelBySoftObjectPtr` "/Game/00/Levels/Lvl_EndMenu.Lvl_EndMenu"))

(fn `UserConstructionScript`)